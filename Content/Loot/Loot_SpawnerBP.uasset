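; Loot spawner Blueprint that spawns a Loot_ItemBP at its own location every second on a looping timer.
; ChooseRarity makes a weighted random roll over the RarityMap in the LootInstance game instance, subtracting each weight until the roll lands.
; GenerateLootScore scales a random base score by a per-rarity multiplier, so Common always scores zero.
; Rarity and rounded score pass to the spawned item as an item struct.
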(event Custom|CreateLoot
  (bind _rarity (CallFunction|ChooseRarity))
  (bind _returnvalue (CallFunction|GenerateLootScore _rarity))
  (Game|SpawnActorfromClass "/Game/Loot/Loot_ItemBP.Loot_ItemBP_C" (Math|Conversions|ToTransform(Vector) (Transformation|GetActorLocation)) "Undefined" 0 (Utilities|Struct|MakeItem_Struct _rarity _returnvalue) 0))

(event EventBeginPlay
  (Utilities|Time|SetTimerbyEvent (delegate Custom|CreateLoot) 1.0 true))

(fn ConstructionScript)

(fn ChooseRarity
  (bind _asloot_instance (Utilities|Casting|CastToLootInstance (Game|GetGameInstance)))
  (bind _keys (Utilities|Map|Keys (Variables|/Game/Loot/LootInstance.LootInstance_C|GetRarityMap _asloot_instance)))
  (for _array_element _keys
    (LocalVariables|SetSomeOfRarities (+ (.Value (Utilities|Map|Find (Variables|/Game/Loot/LootInstance.LootInstance_C|GetRarityMap _asloot_instance) _array_element)) (LocalVariables|GetSomeOfRarities))))
  (LocalVariables|SetLootRool (Math|Random|RandomFloatinRange 0.0 (LocalVariables|GetSomeOfRarities)))
  (bind _keys_2 (Utilities|Map|Keys (Variables|/Game/Loot/LootInstance.LootInstance_C|GetRarityMap _asloot_instance)))
  (bind _array_element_2 (Utilities|Array|ForEachLoopwithBreak _keys_2 :!label _label)
    (:LoopBody
      (if (>= (.Value (Utilities|Map|Find (Variables|/Game/Loot/LootInstance.LootInstance_C|GetRarityMap _asloot_instance) _array_element_2)) (LocalVariables|GetLootRool))
        (LocalVariables|SetRarityOUT _array_element_2)
        (goto _label Break)
        (else
          (LocalVariables|SetLootRool (- (LocalVariables|GetLootRool) (.Value (Utilities|Map|Find (Variables|/Game/Loot/LootInstance.LootInstance_C|GetRarityMap _asloot_instance) _array_element_2)))))))
    (:Completed
      (return (LocalVariables|GetRarityOUT)))))

(fn GenerateLootScore
  (params (Rarity :type Rarity_ENUM%20Enum :default "NewEnumerator0"))
  (LocalVariables|SetLoot%20Score%20Multiplier (Utilities|Select :Index Rarity :NewEnumerator0 0.0 :NewEnumerator1 0.5 :NewEnumerator2 1.0 :NewEnumerator3 1.5 :NewEnumerator4 2.0 :NewEnumerator5 3.0))
  (LocalVariables|SetPreMultiplierScore (Math|Random|RandomFloatinRange 5e+01 2e+02))
  (return (Math|Float|Round (* (LocalVariables|GetLoot%20Score%20Multiplier) (LocalVariables|GetPreMultiplierScore)))))