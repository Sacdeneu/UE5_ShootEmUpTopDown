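; Loot item actor that pops out with a physics impulse and shows a stats widget while looked at.
; The construction script colors the sphere by the item's rarity.
; On BeginPlay the sphere launches upward with random sideways drift, then after a delay stops simulating, becomes query-only and copies loot score, attack, defense and speed into the widget.
; Look events toggle the widget's visibility.
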(event Custom|LookAtItem
  (Rendering|SetVisibility (Variables|Default|GetLoot_UMG) true false))

(event Custom|StopLookingAtItem
  (Rendering|SetVisibility (Variables|Default|GetLoot_UMG) false false))

(event EventBeginPlay
  (bind _itemdetails (Variables|Default|GetItemDetails))
  (bind (_rarity _lootscore _itemstats) (Utilities|Struct|BreakItem_Struct _itemdetails))
  (bind (_attack _defense _speed) (Utilities|Struct|BreakStat_Struct _itemstats))
  (Physics|AddImpulse (Variables|Default|GetSphere) (* (Math|Vector|MakeVector (Math|Random|RandomFloatinRange -0.4 0.4) (Math|Random|RandomFloatinRange -0.4 0.4) 1.0) (Variables|Default|GetImpulseStrength)) "None" false)
  (Utilities|FlowControl|Delay 4.5)
  (Physics|SetSimulatePhysics (Variables|Default|GetSphere) false)
  (Collision|SetCollisionEnabled (Variables|Default|GetSphere) "QueryOnly")
  (bind _asloot_widget_bp (Utilities|Casting|CastToLootWidget_BP (UserInterface|GetUserWidgetObject (Variables|Default|GetLoot_UMG))))
  (Variables|/Game/Loot/LootWidget_BP.LootWidget_BP_C|SetLootScore _asloot_widget_bp _lootscore)
  (Variables|/Game/Loot/LootWidget_BP.LootWidget_BP_C|SetATK_V _asloot_widget_bp _attack)
  (Variables|/Game/Loot/LootWidget_BP.LootWidget_BP_C|SetDEF_V _asloot_widget_bp _defense)
  (Variables|/Game/Loot/LootWidget_BP.LootWidget_BP_C|SetSPD_V _asloot_widget_bp _speed))

(fn ConstructionScript
  (Rendering|Material|SetMaterial (Variables|Default|GetSphere) 0 (Utilities|Select :Index (.Rarity (Utilities|Struct|BreakItem_Struct (Variables|Default|GetItemDetails))) :NewEnumerator0 "/Game/Loot/MI_Grey.MI_Grey" :NewEnumerator1 "/Game/Loot/MI_Solid_Green.MI_Solid_Green" :NewEnumerator2 "/Game/LevelPrototyping/Materials/MI_Solid_Blue.MI_Solid_Blue" :NewEnumerator3 "/Game/Loot/MI_Purple.MI_Purple" :NewEnumerator4 "/Game/Loot/MI_Orange.MI_Orange" :NewEnumerator5 "/Game/Loot/MI_Yellow.MI_Yellow")))